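; OBJ_Cheese is a cheese data object that holds a cheese value and a percent multiplier.
; Each variable has a getter and a setter, and each setter stores the new value, then calls that variable's change notification (CheeseValueHasChanged or PercentMultiplierHasChanged).
; The two values are independent here, with no calculation combining them.
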(fn `GetCheeseValue`
  (returns (CheeseValue :type Integer))
  (return (`self.CheeseValue`)))

(fn `GetPercentMultiplier`
  (returns (PercentMultiplier :type "Float (double-precision)"))
  (return (`self.PercentMultiplier`)))

(fn `SetCheeseValue`
  (params (CheeseValue :type Integer))
  (set `self.CheeseValue` CheeseValue)
  (`self.CheeseValueHasChanged`))

(fn `SetPercentMultiplier`
  (params (PercentMultiplier :type "Float (double-precision)"))
  (set `self.PercentMultiplier` PercentMultiplier)
  (`self.PercentMultiplierHasChanged`))