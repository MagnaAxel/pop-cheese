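; OBJ_News is a news object that carries a percent multiplier and the set of cheese tags the news concerns.
; RandomizePercentMultiplier scales the current PercentMultiplierModifier by a random float within a given range, so repeated calls compound.
; IsCheeseConcerned returns true when a given cheese has at least one of the news item's concerned tags.
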(fn `IsCheeseConcerned`
  (params (Cheese :type "/Game/Dynamic/Blueprints/Cheese/OBJ_Cheese Object Reference"))
  (returns (IsConcerned :type Boolean))
  (bind _result (`BlueprintSetLibrary.Set_ToArray` (`self.CheeseTagsConcerned`)))
  (for _array_element _result
    (if (`BlueprintSetLibrary.Set_Contains` (`/Game/Dynamic/Blueprints/Cheese/OBJ_Cheese.CheeseTags` Cheese) _array_element)
      (return true)))
  (return false))

(fn `RandomizePercentMultiplier`
  (params (MinMultiplier :type "Float (double-precision)" :default 1.0) (MaxMultiplier :type "Float (double-precision)" :default 3.0))
  (set `self.PercentMultiplierModifier` (* (`KismetMathLibrary.RandomFloatInRange` MinMultiplier MaxMultiplier) (`self.PercentMultiplierModifier`))))