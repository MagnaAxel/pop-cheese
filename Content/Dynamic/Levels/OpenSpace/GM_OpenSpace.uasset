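; Game mode for the OpenSpace level that spawns players and runs a timed, looping cheese-investment economy.
; Timers chain News, Invest, Flow and Reward phases, switching player UI focus and adding unique random cheeses to GameState on set turns.
; Random news shifts matching cheeses' percent multipliers during Flow, banking gains in the GameState total or shrinking cheese values.
; Reward only checks that total against the win threshold and prints a message.
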(event `self.K2_PostLogin`
  (params (NewPlayer :type "PlayerController Object Reference"))
  (bind _returnvalue (`|SpawnActorFromClass` "/Game/Dynamic/Blueprints/Player/BP_Player.BP_Player_C" (`self.GetTransform` (`self.K2_FindPlayerStart` NewPlayer)) "Undefined" "MultiplyWithRoot" null null))
  (`Controller.Possess` NewPlayer _returnvalue)
  (`self.StartPhase`))

(event `StartPhase`
  (`self.IncrementTurn`)
  (`self.NewsPhase`))

(event `NewsPhase`
  (bind _returnvalue (`KismetSystemLibrary.K2_SetTimerDelegate` (delegate `InvestPhase`) (`self.NewsTimer`)))
  (set `self.ActiveTimer` _returnvalue)
  (`self.ChooseNews`)
  (`self.FocusNews`)
  (`KismetSystemLibrary.PrintString` "NewsPhase"))

(event `InvestPhase`
  (bind _returnvalue (`KismetSystemLibrary.K2_SetTimerDelegate` (delegate `FlowEvent`) (`self.InvestTimer`)))
  (set `self.ActiveTimer` _returnvalue)
  (`self.FocusInvest`)
  (`KismetSystemLibrary.PrintString` "InvestPhase"))

(event `FlowEvent`
  (bind _returnvalue (`KismetSystemLibrary.K2_SetTimerDelegate` (delegate `RewardEvent`) (`self.FlowTimer`)))
  (set `self.ActiveTimer` _returnvalue)
  (`self.PlayFlow`)
  (`KismetSystemLibrary.PrintString` "FlowPhase"))

(event `RewardEvent`
  (bind _returnvalue (`KismetSystemLibrary.K2_SetTimerDelegate` (delegate `StartPhase`) (`self.RewardTimer`)))
  (set `self.ActiveTimer` _returnvalue)
  (`self.GiveReward`)
  (`KismetSystemLibrary.PrintString` "RewardPhase"))

(fn `AddCheese`
  (params (Quantity :type Integer))
  (locals (ChosenCheese :type "/Game/Dynamic/Blueprints/Cheese/OBJ_Cheese Class Reference"))
  (bind _cheeseclasses (`self.CheeseClasses`))
  (for _ (range 1 (+ Quantity 1))
    (bind _output_get (set `local.ChosenCheese` (`|GetArrayItem` _cheeseclasses (`KismetMathLibrary.RandomIntegerInRange` 0 (- (`KismetArrayLibrary.Array_Length` _cheeseclasses) 1)))))
    (bind _returnvalue (`|GenericCreateObject` _output_get))
    (bind _asgs_open_space (cast `/Game/Dynamic/Levels/OpenSpace/GS_OpenSpace` (`GameplayStatics.GetGameState`)))
    (`KismetArrayLibrary.Array_AddUnique` (`/Game/Dynamic/Levels/OpenSpace/GS_OpenSpace.Cheeses` _asgs_open_space) _returnvalue)
    (`KismetArrayLibrary.Array_RemoveItem` (`self.CheeseClasses`) (`local.ChosenCheese`))))

(fn `ChooseNews`
  (locals (News :type "/Game/Dynamic/Blueprints/News/OBJ_News Object Reference"))
  (bind _newsclasses (`self.NewsClasses`))
  (bind _asgs_open_space (cast `/Game/Dynamic/Levels/OpenSpace/GS_OpenSpace` (`GameplayStatics.GetGameState`)))
  (`/Game/Dynamic/Levels/OpenSpace/GS_OpenSpace.ClearNews` _asgs_open_space)
  (for _ (range (+ (`KismetMathLibrary.RandomIntegerInRange` 1 3) 1))
    (bind _returnvalue (`|GenericCreateObject` (`|GetArrayItem` _newsclasses (`KismetMathLibrary.RandomIntegerInRange` 0 (- (`KismetArrayLibrary.Array_Length` _newsclasses) 1)))))
    (bind _output_get (set `local.News` _returnvalue))
    (`/Game/Dynamic/Blueprints/News/OBJ_News.RandomizePercentMultiplier` _output_get 1.0 3.0)
    (bind _asgs_open_space_2 (cast `/Game/Dynamic/Levels/OpenSpace/GS_OpenSpace` (`GameplayStatics.GetGameState`)))
    (`/Game/Dynamic/Levels/OpenSpace/GS_OpenSpace.AddNews` _asgs_open_space_2 (`local.News`))))

(fn `FocusInvest`
  (bind _aspc_open_space (cast `/Game/Dynamic/Blueprints/Player/PC_OpenSpace` (`GameplayStatics.GetPlayerController` 0)))
  (`/Game/Dynamic/Blueprints/Player/WI_Interface.FocusInvest` (`/Game/Dynamic/Blueprints/Player/PC_OpenSpace.Interface` _aspc_open_space)))

(fn `FocusNews`
  (bind _aspc_open_space (cast `/Game/Dynamic/Blueprints/Player/PC_OpenSpace` (`GameplayStatics.GetPlayerController` 0)))
  (`/Game/Dynamic/Blueprints/Player/WI_Interface.FocusNews` (`/Game/Dynamic/Blueprints/Player/PC_OpenSpace.Interface` _aspc_open_space)))

(fn `GiveReward`
  (bind _asgs_open_space (cast `/Game/Dynamic/Levels/OpenSpace/GS_OpenSpace` (`GameplayStatics.GetGameState`)))
  (bind _cheesevalue (`/Game/Dynamic/Levels/OpenSpace/GS_OpenSpace.GetCheeseValue` _asgs_open_space))
  (if (>= _cheesevalue (`/Game/Dynamic/Levels/OpenSpace/GS_OpenSpace.WinCheeseValue` _asgs_open_space))
    (`KismetSystemLibrary.PrintString` "YouWin")))

(fn `IncrementTurn`
  (bind _asgs_open_space (cast `/Game/Dynamic/Levels/OpenSpace/GS_OpenSpace` (`GameplayStatics.GetGameState`)))
  (bind _turn (`/Game/Dynamic/Levels/OpenSpace/GS_OpenSpace.GetTurn` _asgs_open_space))
  (bind _result (`/Engine/EditorBlueprintResources/StandardMacros.IncrementInt` _turn)
    (:`  `
      (`/Game/Dynamic/Levels/OpenSpace/GS_OpenSpace.SetTurn` _asgs_open_space _result)
      (if (`BlueprintSetLibrary.Set_Contains` (`self.AddCheeseTurn`) _result)
        (if (== _result 1)
          (`self.AddCheese` 4)
          (else
            (`self.AddCheese` 2)))))))

(fn `PlayFlow`
  (locals (CheeseFlowValue :type "Float (double-precision)"))
  (`|ExecutionSequence`
    (:`then_0`
      (bind _asgs_open_space (cast `/Game/Dynamic/Levels/OpenSpace/GS_OpenSpace` (`GameplayStatics.GetGameState`)))
      (bind _news (`/Game/Dynamic/Levels/OpenSpace/GS_OpenSpace.GetNews` _asgs_open_space))
      (for _array_element _news
        (for _array_element_2 (`/Game/Dynamic/Levels/OpenSpace/GS_OpenSpace.Cheeses` _asgs_open_space)
          (bind _isconcerned (`/Game/Dynamic/Blueprints/News/OBJ_News.IsCheeseConcerned` _array_element _array_element_2))
          (if _isconcerned
            (bind _percentmultiplier (`/Game/Dynamic/Blueprints/Cheese/OBJ_Cheese.GetPercentMultiplier` _array_element_2))
            (`/Game/Dynamic/Blueprints/Cheese/OBJ_Cheese.SetPercentMultiplier` _array_element_2 (+ (`/Game/Dynamic/Blueprints/News/OBJ_News.PercentMultiplierModifier` _array_element) _percentmultiplier))))))
    (:`then_1`
      (bind _asgs_open_space_2 (cast `/Game/Dynamic/Levels/OpenSpace/GS_OpenSpace` (`GameplayStatics.GetGameState`)))
      (for _array_element_3 (`/Game/Dynamic/Levels/OpenSpace/GS_OpenSpace.Cheeses` _asgs_open_space_2)
        (bind _percentmultiplier_2 (`/Game/Dynamic/Blueprints/Cheese/OBJ_Cheese.GetPercentMultiplier` _array_element_3))
        (bind _cheesevalue (`/Game/Dynamic/Blueprints/Cheese/OBJ_Cheese.GetCheeseValue` _array_element_3))
        (bind _output_get (set `local.CheeseFlowValue` (* (* _percentmultiplier_2 0.01) _cheesevalue)))
        (if (>= _output_get _cheesevalue)
          (bind _cheesevalue_2 (`/Game/Dynamic/Blueprints/Cheese/OBJ_Cheese.GetCheeseValue` _array_element_3))
          (bind _asgs_open_space_3 (cast `/Game/Dynamic/Levels/OpenSpace/GS_OpenSpace` (`GameplayStatics.GetGameState`)))
          (bind _cheesevalue_3 (`/Game/Dynamic/Levels/OpenSpace/GS_OpenSpace.GetCheeseValue` _asgs_open_space_3))
          (`/Game/Dynamic/Levels/OpenSpace/GS_OpenSpace.SetCheeseValue` _asgs_open_space_3 (+ _cheesevalue_3 (- (`local.CheeseFlowValue`) _cheesevalue_2)))
          (else
            (`/Game/Dynamic/Blueprints/Cheese/OBJ_Cheese.SetCheeseValue` _array_element_3 (`KismetMathLibrary.FTrunc` (`local.CheeseFlowValue`)))))))))

(fn `UserConstructionScript`)